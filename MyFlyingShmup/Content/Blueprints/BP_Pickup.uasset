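; BP_Pickup is a pickup actor that can fly to the player and notify whatever actor it overlaps.
; ActivatePickupHoming turns its ProjectileMovement into a homing projectile aimed at the first player pawn's root component, with a raised speed cap.
; On any overlap it sends the ActivatePickupPowers message to the other actor, leaving the effect to the receiver.
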(event `/Game/Core/BPI_MyFlyingVehicle.ActivatePickupHoming`
  (set `ProjectileMovementComponent.HomingTargetComponent` (`Actor.RootComponent` (`GameplayStatics.GetPlayerPawn` 0)) (`self.ProjectileMovement`))
  (set `ProjectileMovementComponent.bIsHomingProjectile` true (`self.ProjectileMovement`))
  (set `ProjectileMovementComponent.MaxSpeed` 6400.0 (`self.ProjectileMovement`)))

(event `self.ReceiveActorBeginOverlap`
  (params (OtherActor :type "Actor Object Reference"))
  (message `/Game/Core/BPI_MyFlyingVehicle.ActivatePickupPowers` OtherActor))

(fn `GetTitleColor`
  (returns (ReturnValue :type "LinearColor Structure"))
  (return))

(fn `UserConstructionScript`)