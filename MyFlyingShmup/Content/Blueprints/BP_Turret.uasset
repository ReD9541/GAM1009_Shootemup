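; BP_Turret is an enemy turret that fires bullet projectiles at a fixed interval.
; A looping timer started on BeginPlay spawns BP_Projectile_Bullet_Enemy at the Arrow component's transform and plays a 2D gunshot sound.
; When AutoAim is set, Tick yaws the Cylinder mesh toward the player pawn, ignoring pitch and roll.
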(event `self.ReceiveBeginPlay`
  (`KismetSystemLibrary.K2_SetTimerDelegate` (delegate `ShootBullet`) 2.0 true true))

(event `ShootBullet`
  (bind _arrow (`self.Arrow`))
  ; Shoot Bullet
  (`|SpawnActorFromClass` "/Game/Blueprints/BP_Projectile_Bullet_Enemy.BP_Projectile_Bullet_Enemy_C" (`KismetMathLibrary.MakeTransform` (`SceneComponent.K2_GetComponentLocation` _arrow) (`SceneComponent.K2_GetComponentRotation` _arrow)) "Undefined" "MultiplyWithRoot" null null)
  (`GameplayStatics.PlaySound2D` "/Game/FreeWeaponSFX/Cue/AssaultRifle/Gunshots/sfx_wpn_ar_gunshot_01_Cue.sfx_wpn_ar_gunshot_01_Cue" 0.05 1.0 0.0 null null))

(event `self.ReceiveTick`
  (params (DeltaSeconds :type "Float (single-precision)"))
  (bind (_returnvalue_roll _returnvalue_pitch _returnvalue_yaw) (`KismetMathLibrary.BreakRotator` (`KismetMathLibrary.FindLookAtRotation` (`self.K2_GetActorLocation`) (`self.K2_GetActorLocation` (`GameplayStatics.GetPlayerPawn` 0)))))
  (if (`self.AutoAim`)
    (`SceneComponent.K2_SetWorldRotation` (`self.Cylinder`) (`KismetMathLibrary.MakeRotator` 0.0 0.0 _returnvalue_yaw) false false)))

(fn `UserConstructionScript`)