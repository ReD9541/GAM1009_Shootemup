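; BP_Projectile is a projectile actor that damages whatever it overlaps and then destroys itself.
; On overlap it applies its Damage variable to the other actor, passing its instigator controller and itself as damage causer.
; A second damage-and-destroy branch that checks Instigator validity is never executed, and the construction script is empty.
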(event `self.ReceiveActorBeginOverlap`
  (params (OtherActor :type "Actor Object Reference"))
  (`GameplayStatics.ApplyDamage` OtherActor (`self.Damage`) (`self.GetInstigatorController`) self)
  (`self.K2_DestroyActor`))

(fn `UserConstructionScript`)