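; Player-driven tank actor that enables input from player controller 0 to drive, steer and turn its turret.
; W/S, A/D and Q/E open and close gates that Tick feeds through a sequence.
; Open gates apply fixed per-frame steps, unscaled by delta time: swept local movement, body yaw or Head yaw.
; The four wheels spin with travel and counter-rotate in pairs during turns.
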(event `self.ReceiveBeginPlay`
  ;[0.1475 0.15 0.0517 0.5] Enables inputs
  (`self.EnableInput` (`GameplayStatics.GetPlayerController` 0)))

(event `Key|W`
  (params (Key :type "Key Structure"))
  ;[0.15 0.111 0.005469 0.5] Move Forward and Backwards
  (:`Pressed`
    (goto _label :!via `Open`))
  (:`Released`
    (goto _label :!via `Close`)))

(event `Key|S`
  (params (Key :type "Key Structure"))
  ;[0.15 0.111 0.005469 0.5] Move Forward and Backwards
  (:`Pressed`
    (goto _label_2 :!via `Open`))
  (:`Released`
    (goto _label_2 :!via `Close`)))

(event `self.ReceiveTick`
  (params (DeltaSeconds :type "Float (single-precision)"))
  (bind _head (`self.Head`))
  (bind _wheel2 (`self.Wheel2`))
  (`|ExecutionSequence`
    (:`then_0`
      ;[0.15 0.111 0.005469 0.5] Move Forward and Backwards
      (`/Engine/EditorBlueprintResources/StandardMacros.Gate` true :!label _label
        (:`Exit`
          (`self.K2_AddActorLocalOffset` (1.0 0.0 0.0) true)
          ;[0.15 0.5565 0.005469 0.5] Rotate wheels When moving
          (`SceneComponent.K2_AddLocalRotation` _wheel2 (struct :`Pitch` -3.0) false false)
          (`SceneComponent.K2_AddLocalRotation` (`self.Wheel3`) (struct :`Pitch` -3.0) false false)
          (`SceneComponent.K2_AddLocalRotation` (`self.Wheel4`) (struct :`Pitch` -3.0) false false)
          (`SceneComponent.K2_AddLocalRotation` (`self.Wheel1`) (struct :`Pitch` -3.0) false false))))
    (:`then_1`
      (`/Engine/EditorBlueprintResources/StandardMacros.Gate` true :!label _label_2
        (:`Exit`
          (`self.K2_AddActorLocalOffset` (-1.0 0.0 0.0) true)
          (`SceneComponent.K2_AddLocalRotation` _wheel2 (struct :`Pitch` 3.0) false false)
          (`SceneComponent.K2_AddLocalRotation` (`self.Wheel3`) (struct :`Pitch` 3.0) false false)
          (`SceneComponent.K2_AddLocalRotation` (`self.Wheel4`) (struct :`Pitch` 3.0) false false)
          (`SceneComponent.K2_AddLocalRotation` (`self.Wheel1`) (struct :`Pitch` 3.0) false false))))
    (:`then_2`
      ;[0.15 0.111 0.005469 0.5] Rotate Entire Tank
      (`/Engine/EditorBlueprintResources/StandardMacros.Gate` true :!label _label_3
        (:`Exit`
          (`self.K2_AddActorWorldRotation` (struct :`Yaw` -1.0))
          ;[0.15 0.5565 0.005469 0.5] Rotate Wheels and tank Rotates
          (`SceneComponent.K2_AddLocalRotation` (`self.Wheel1`) (struct :`Pitch` -3.0) false false)
          (`SceneComponent.K2_AddLocalRotation` (`self.Wheel2`) (struct :`Pitch` -3.0) false false)
          (`SceneComponent.K2_AddLocalRotation` (`self.Wheel3`) (struct :`Pitch` 3.0) false false)
          (`SceneComponent.K2_AddLocalRotation` (`self.Wheel4`) (struct :`Pitch` 3.0) false false))))
    (:`then_3`
      (`/Engine/EditorBlueprintResources/StandardMacros.Gate` true :!label _label_4
        (:`Exit`
          (`self.K2_AddActorWorldRotation` (struct :`Yaw` 1.0))
          (`SceneComponent.K2_AddLocalRotation` (`self.Wheel1`) (struct :`Pitch` 3.0) false false)
          (`SceneComponent.K2_AddLocalRotation` (`self.Wheel2`) (struct :`Pitch` 3.0) false false)
          (`SceneComponent.K2_AddLocalRotation` (`self.Wheel3`) (struct :`Pitch` -3.0) false false)
          (`SceneComponent.K2_AddLocalRotation` (`self.Wheel4`) (struct :`Pitch` -3.0) false false))))
    (:`then_4`
      ;[0.15 0.111 0.005469 0.5] Rotates the head/canon
      (`/Engine/EditorBlueprintResources/StandardMacros.Gate` true :!label _label_5
        (:`Exit`
          (`SceneComponent.K2_AddLocalRotation` _head (struct :`Yaw` -1.0) false false))))
    (:`then_5`
      (`/Engine/EditorBlueprintResources/StandardMacros.Gate` true :!label _label_6
        (:`Exit`
          (`SceneComponent.K2_AddLocalRotation` _head (struct :`Yaw` 1.0) false false))))))

(event `Key|A`
  (params (Key :type "Key Structure"))
  ;[0.15 0.111 0.005469 0.5] Rotate Entire Tank
  (:`Pressed`
    (goto _label_3 :!via `Open`))
  (:`Released`
    (goto _label_3 :!via `Close`)))

(event `Key|D`
  (params (Key :type "Key Structure"))
  ;[0.15 0.111 0.005469 0.5] Rotate Entire Tank
  (:`Pressed`
    (goto _label_4 :!via `Open`))
  (:`Released`
    (goto _label_4 :!via `Close`)))

(event `Key|Q`
  (params (Key :type "Key Structure"))
  ;[0.15 0.111 0.005469 0.5] Rotates the head/canon
  (:`Pressed`
    (goto _label_5 :!via `Open`))
  (:`Released`
    (goto _label_5 :!via `Close`)))

(event `Key|E`
  (params (Key :type "Key Structure"))
  ;[0.15 0.111 0.005469 0.5] Rotates the head/canon
  (:`Pressed`
    (goto _label_6 :!via `Open`))
  (:`Released`
    (goto _label_6 :!via `Close`)))

(fn `UserConstructionScript`)