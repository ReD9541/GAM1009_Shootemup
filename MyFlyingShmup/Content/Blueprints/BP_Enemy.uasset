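; Enemy actor that deals its max health as damage to any actor it overlaps and may carry a turret.
; On spawn it randomly attaches a BP_Turret with random auto-aim, destroyed along with the enemy.
; Incoming damage awards score to the instigator via message, flashes an overlay material with sound, and updates the health bar widget.
; At zero health it plays a sound, spawns an explosion and destroys itself.
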(event `self.ReceiveDestroyed`
  ; Destroy spawned attached turret
  (bind _spawnedturret (`self.SpawnedTurret`)
    (:`then`
      (`self.K2_DestroyActor` _spawnedturret))
    (:`else`)))

(event `SpawnTurret`
  ; Spawn Turret
  (if (< (`KismetMathLibrary.RandomFloat`) 0.2)
    (bind _returnvalue (`|SpawnActorFromClass` "/Game/Blueprints/BP_Turret.BP_Turret_C" (`KismetMathLibrary.MakeTransform` (`SceneComponent.K2_GetComponentLocation` (`self.TurretAttachPoint`))) "Undefined" "MultiplyWithRoot" null (`KismetMathLibrary.RandomBool`) null))
    (bind _output_get (set `self.SpawnedTurret` _returnvalue))
    (`self.K2_AttachToComponent` _output_get (`self.TurretAttachPoint`) "None" "SnapToTarget" "KeepRelative" "KeepRelative" false)))

(event `self.ReceiveBeginPlay`
  ; Initialize health
  (set `self.Health` (`self.MaxHealth`))
  (`self.SetWidgetHealth`)
  (`self.SpawnTurret`))

(event `self.ReceiveActorBeginOverlap`
  (params (OtherActor :type "Actor Object Reference"))
  (`GameplayStatics.ApplyDamage` OtherActor (`self.MaxHealth`)))

(event `DeathSequence`
  ; Death Sequence
  (`GameplayStatics.PlaySound2D` "/Game/FreeWeaponSFX/Cue/Handgun/Gunshots/sfx_wpn_hgn_tail_01_Cue.sfx_wpn_hgn_tail_01_Cue" 2.0 1.0 0.0 null null)
  (`|SpawnActorFromClass` "/Game/VFX/BP_Explosion.BP_Explosion_C" (`KismetMathLibrary.MakeTransform` (`self.K2_GetActorLocation`) (`self.K2_GetActorRotation`)) "Undefined" "MultiplyWithRoot" null null)
  (`KismetSystemLibrary.DelayUntilNextFrame`)
  (`self.K2_DestroyActor`))

(event `ApplyDamageAsScore`
  (params (Points :type "Float (double-precision)"))
  ; Update Player Score
  (bind _instigated_by (`self.Instigated By`)
    (:`then`
      (message `/Game/Core/BPI_MyFlyingVehicle.AddScore` _instigated_by Points))
    (:`else`)))

(event `HitSequence`
  ; Hit Sequence
  (`GameplayStatics.PlaySound2D` "/Game/FreeWeaponSFX/Cue/AssaultRifle/Gunshots/sfx_wpn_ar_tail_01_Cue.sfx_wpn_ar_tail_01_Cue" 1.0 1.0 0.0 null null)
  (`self.HitEffects`))

(event `HitEffects`
  ; Hit effects
  (`MeshComponent.SetOverlayMaterial` (`self.StaticMesh`) "/Game/Materials/MI_Overlay_HitEffect_White.MI_Overlay_HitEffect_White" false 0)
  (`KismetSystemLibrary.Delay` 0.2)
  (`MeshComponent.SetOverlayMaterial` (`self.StaticMesh`) null false 0))

(event `self.ReceiveAnyDamage`
  (params (Damage :type "Float (single-precision)") (DamageType :type "DamageType Object Reference") (InstigatedBy :type "Controller Object Reference") (DamageCauser :type "Actor Object Reference"))
  ; Deal Damage and Recalculate Health
  (set `self.Instigated By` InstigatedBy)
  (`self.ApplyDamageAsScore` Damage)
  (`self.HitSequence`)
  (bind _output_get (set `self.Health` (`KismetMathLibrary.FMax` (- (`self.Health`) Damage))))
  (`self.SetWidgetHealth`)
  (if (== _output_get 0.0)
    (`self.DeathSequence`)))

(event `SetWidgetHealth`
  ; Widget Health
  (message `/Game/Core/BPI_MyFlyingVehicle.SetEnemyHealthBar` (`WidgetComponent.GetUserWidgetObject` (`self.Widget`)) (`KismetMathLibrary.SafeDivide` (`self.Health`) (`self.MaxHealth`)) (`self.Health`)))

(fn `UserConstructionScript`)