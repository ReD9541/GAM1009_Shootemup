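; Simple enemy spawner actor that keeps spawning random enemies along a line for as long as it runs.
; BeginPlay starts a randomly timed one-shot timer, which each spawn re-arms with a fresh delay.
; Each spawn picks one of three enemy classes and places it at a random Y between two arrow components, using the right arrow's X and Z and the spawner's rotation, ignoring collisions.
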(event `self.ReceiveBeginPlay`
  (`self.StartTimer`))

(event `StartTimer`
  ; Timer
  (`KismetSystemLibrary.K2_SetTimerDelegate` (delegate `SpawnEnemy`) (`KismetMathLibrary.RandomFloatInRange` 2.0 4.0) false true))

(event `SpawnEnemy`
  (bind (_returnvalue_x _returnvalue_y) (`KismetMathLibrary.BreakVector` (`SceneComponent.K2_GetComponentLocation` (`self.ArrowLeft`))))
  (bind (_returnvalue_x_2 _returnvalue_y_2 _returnvalue_z) (`KismetMathLibrary.BreakVector` (`SceneComponent.K2_GetComponentLocation` (`self.ArrowRight`))))
  ; Spawning Enemies
  (`|SpawnActorFromClass` (`KismetArrayLibrary.Array_Random` (`|MakeArray` "/Game/Blueprints/BP_Enemy_1.BP_Enemy_1_C" "/Game/Blueprints/BP_Enemy_2.BP_Enemy_2_C" "/Game/Blueprints/BP_Enemy_3.BP_Enemy_3_C" :!type "Actor Class Reference")) (`KismetMathLibrary.MakeTransform` (`KismetMathLibrary.MakeVector` _returnvalue_x_2 (`KismetMathLibrary.RandomFloatInRange` _returnvalue_y_2 _returnvalue_y) _returnvalue_z) (`self.K2_GetActorRotation`)) "AlwaysSpawn" "MultiplyWithRoot")
  (`self.StartTimer`))

(fn `UserConstructionScript`)